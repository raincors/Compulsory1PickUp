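; BP_MyFPSCharacter is a first-person character Blueprint that triggers item pickups and sets up a HUD with a ring count.
; On BeginPlay it creates WBP_HUD, adds it to the viewport and resets the ring count shown in its counter widget to zero.
; Capsule hits against a BP_Interactable call PickUp with the character as argument, leaving the pickup logic and any count increase outside this Blueprint.
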(event `self.ReceiveBeginPlay`
  (bind _returnvalue (`|CreateWidget` "/Game/Widgets/WBP_HUD.WBP_HUD_C"))
  (bind _output_get (set `self.HUD` _returnvalue))
  (`UserWidget.AddToViewport` _output_get 0)
  (bind _output_get_2 (set `self.RingNumber` 0))
  (`/Game/Widgets/WBP_RingCount.UpdateItemsCount` (`/Game/Widgets/WBP_HUD.WBP_RingCount` (`self.HUD`)) _output_get_2))

(event `self.ReceiveActorBeginOverlap`
  (params (OtherActor :type "Actor Object Reference")))

(event `self.CapsuleComponent.OnComponentHit`
  (params (HitComponent :type "PrimitiveComponent Object Reference") (OtherActor :type "Actor Object Reference") (OtherComp :type "PrimitiveComponent Object Reference") (NormalImpulse :type "Vector Structure") (Hit :type "HitResult Structure (by ref)"))
  (bind _asbp_interactable (cast `/Game/Blueprints/BP_Interactable` OtherActor))
  (`/Game/Blueprints/BP_Interactable.PickUp` _asbp_interactable self))

(fn `UserConstructionScript`)